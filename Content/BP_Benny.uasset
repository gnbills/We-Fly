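; BP_Benny is a Paper2D sprite actor, Benny, that patrols back and forth, reversing direction when its sprite registers a hit.
; Every Tick, Move offsets the actor location by the MovementSpeed vector, without sweep or delta-time scaling.
; The sprite's OnComponentHit calls FlipMovement, which swaps the left or right facing sprite, negates MovementSpeed and toggles IsMovingLeft.
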(event OnComponentHit(PaperSprite)
  (params (HitComponent :type Primitive%20Component%20Object%20Reference) (OtherActor :type Actor%20Object%20Reference) (OtherComp :type Primitive%20Component%20Object%20Reference) (NormalImpulse :type Vector :default "0, 0, 0") (Hit :type Hit%20Result%20Structure%20%28by%20ref%29))
  (CallFunction|FlipMovement))

(event EventBeginPlay)

(event EventTick
  (params (DeltaSeconds :type Float%20%28single-precision%29))
  (CallFunction|Move))

(fn ConstructionScript)

(fn Move
  (Transformation|SetActorLocation (+ (Variables|Default|GetMovement_Speed) (Transformation|GetActorLocation)) false false))

(fn FlipMovement
  (if (Variables|Default|GetIs_Moving_Left)
    (Rendering|Components|Sprite|SetSprite (Variables|Default|GetPaperSprite) "/Game/Sprites/Benny_Right_Sprite.Benny_Right_Sprite")
    (else
      (Rendering|Components|Sprite|SetSprite (Variables|Default|GetPaperSprite) "/Game/Sprites/Benny_Left_Sprite.Benny_Left_Sprite")))
  (Variables|Default|SetMovement_Speed (Math|Vector|NegateVector (Variables|Default|GetMovement_Speed)))
  (Variables|Default|SetIs_Moving_Left (not (Variables|Default|GetIs_Moving_Left))))