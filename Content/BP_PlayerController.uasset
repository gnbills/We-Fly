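; BP_PlayerController is the player controller that turns keyboard presses into movement commands for the controlled BP_Player pawn.
; W, A and D each cast the controlled pawn to BP_Player and call its Move with a directional force and an Up, Left or Right state.
; The controller's own Move function and construction script are empty, so the pawn handles the actual movement.
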(event Input|KeyboardEvents|W
  (params (Key :type Key%20Structure))
  (:Pressed
    (bind _asbp_player (Utilities|Casting|CastToBP_Player (Pawn|GetControlledPawn)))
    (Default|Move _asbp_player (Variables|Default|GetUpward%20Force) "Up")))

(event Input|KeyboardEvents|A
  (params (Key :type Key%20Structure))
  (:Pressed
    (bind _asbp_player (Utilities|Casting|CastToBP_Player (Pawn|GetControlledPawn)))
    (Default|Move _asbp_player (Variables|Default|GetForce%20From%20Right) "Left")))

(event Input|KeyboardEvents|D
  (params (Key :type Key%20Structure))
  (:Pressed
    (bind _asbp_player (Utilities|Casting|CastToBP_Player (Pawn|GetControlledPawn)))
    (Default|Move _asbp_player (Variables|Default|GetForce%20From%20Left) "Right")))

(fn ConstructionScript)

(fn Move
  (params (Force :type Vector)))