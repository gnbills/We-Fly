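; Player actor for a cardinal bird that the player guides to a nest, with a timer for the run.
; Move applies physics impulses to the sprite, swapping left and right art on direction changes.
; Tick uses a Delay to count seconds until Win, which saves the time to the game instance and opens the victory level.
; Die shows the lose screen and cursor, then destroys the actor.
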(event Custom|Win
  (Audio|PlaySound2D "/Game/Music_and_Sound/Jingle_Nest.Jingle_Nest")
  (Variables|Default|SetHasn't_Nested false)
  (bind _asmy_game_instance (Utilities|Casting|CastToMy_Game_Instance (Game|GetGameInstance)))
  (Variables|/Game/My_Game_Instance.My_Game_Instance_C|SetTime _asmy_game_instance (Variables|Default|GetTime))
  (Utilities|FlowControl|Delay 1.5)
  (Game|OpenLevel(byName) "Victory_Screen"))

(event EventBeginPlay)

(event Collision|EventActorBeginOverlap
  (params (OtherActor :type Actor%20Object%20Reference)))

(event EventTick
  (params (DeltaSeconds :type Float%20%28single-precision%29))
  (if (Variables|Default|GetHasn't_Nested)
    (Utilities|FlowControl|Delay 1.0)
    (Variables|Default|SetTime (+ (Variables|Default|GetTime) (Math|Timespan|MakeTimespan 0 0 0 1)))))

(fn ConstructionScript)

(fn Move
  (params (Force :type Vector) (State :type String))
  (switch string State
    (:Up
      (Physics|AddImpulse (Variables|Default|GetCardinal_Sprite) Force "None" false))
    (:Left
      (if (Variables|Default|GetAlready_Moving_Left)
        _
        (else
          (Rendering|Components|Sprite|SetSprite (Variables|Default|GetCardinal_Sprite) "/Game/Sprites/Cardinal_Left_Sprite.Cardinal_Left_Sprite")
          (Variables|Default|SetAlready_Moving_Left true)))
      (Physics|AddImpulse (Variables|Default|GetCardinal_Sprite) Force "None" false))
    (:Right
      (if (Variables|Default|GetAlready_Moving_Left)
        (Rendering|Components|Sprite|SetSprite (Variables|Default|GetCardinal_Sprite) "/Game/Sprites/Cardinal_Right_Sprite.Cardinal_Right_Sprite")
        (Variables|Default|SetAlready_Moving_Left false))
      (Physics|AddImpulse (Variables|Default|GetCardinal_Sprite) Force "None" false))))

(fn FlipSprite
  (Rendering|Components|Sprite|SetSprite (Variables|Default|GetCardinal_Sprite) "/Game/Sprites/Cardinal_Right_Sprite.Cardinal_Right_Sprite"))

(fn Die
  (bind _returnvalue (UserInterface|CreateWidget "/Game/Widgets/Lose_Screen.Lose_Screen_C" (Game|GetPlayerController 0)))
  (UserInterface|Viewport|AddtoViewport _returnvalue 0)
  (Variables|/Script/Engine.PlayerController|SetbShowMouseCursor (Game|GetPlayerController 0) true)
  (Actor|DestroyActor))

(fn GetPlayerHeight
  (return (.Z (Math|Vector|BreakVector (Transformation|GetWorldLocation (Variables|Default|GetCardinal_Sprite))))))